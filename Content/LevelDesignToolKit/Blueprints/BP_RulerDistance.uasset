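; BP_RulerDistance is a level design ruler that shows the distance between its spline mesh origin and an end point, plus a description label.
; The Construction Script places a marker at EndPoint, aims the spline mesh and end cylinder along that line, and stretches the mesh by a scaled distance.
; It writes the rounded distance and Description to text components.
; The Event Graph holds only disabled stubs, so nothing runs on Tick.
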(event EventBeginPlay)

(event Collision|EventActorBeginOverlap
  (params (OtherActor :type Actor%20Object%20Reference)))

(event EventTick
  (params (DeltaSeconds :type Float%20%28single-precision%29)))

(fn ConstructionScript
  (bind _splinemesh (Variables|Default|GetSplineMesh))
  (bind _endpointloccube (Variables|Default|GetEndPointLocCube))
  (bind _returnvalue (Transformation|GetWorldLocation _splinemesh))
  (bind _returnvalue_2 (Transformation|GetWorldLocation _endpointloccube))
  (bind _returnvalue_3 (Math|Vector|Distance(Vector) _returnvalue _returnvalue_2))
  (bind _returnvalue_4 (Math|Rotator|FindLookatRotation _returnvalue _returnvalue_2))
  (Transformation|SetRelativeLocation (Variables|Default|GetEndPointLocCube) (Variables|Default|GetEndPoint) false false)
  (Transformation|SetWorldRotation _splinemesh (Math|Rotator|MakeRotator (.roll _returnvalue_4) (.pitch _returnvalue_4) (.yaw _returnvalue_4)) false false)
  (Transformation|SetWorldRotation (Variables|Default|GetCylinderEnd) (Math|Rotator|MakeRotator (.roll _returnvalue_4) (+ (.pitch _returnvalue_4) -9e+01) (.yaw _returnvalue_4)) false false)
  (SplineMesh|SetEndPosition _splinemesh (Math|Vector|MakeVector (* _returnvalue_3 2e+01) 0.0 0.0) true)
  (Rendering|Components|TextRender|SetText (Variables|Default|GetTextDistance) (Utilities|Text|ToText(Float) (Math|Conversions|ToFloat(Integer) (Math|Float|Round _returnvalue_3)) "HalfToEven"))
  (Rendering|Components|TextRender|SetText (Variables|Default|GetTextDesc) (Variables|Default|GetDescription)))