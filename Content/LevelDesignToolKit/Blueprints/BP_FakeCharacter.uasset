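; BP_FakeCharacter is a Level Design Toolkit actor that shows a character-sized stand-in mesh labeled with its size in centimeters.
; The construction script uniformly scales the static mesh by the ratio of SizeInCm to the mesh's real size.
; It also moves a text render to that height and sets its text to the size; the event graph holds no active logic.
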(event EventBeginPlay)

(event Collision|EventActorBeginOverlap
  (params (OtherActor :type Actor%20Object%20Reference)))

(event EventTick
  (params (DeltaSeconds :type Float%20%28single-precision%29)))

(fn ConstructionScript
  (Transformation|SetRelativeScale3D (Variables|Default|GetStaticMesh) (Math|Conversions|ToVector(Float) (/ (Variables|Default|GetSizeInCm) (Variables|Default|GetStaticMeshRealSize))))
  (Transformation|SetRelativeLocation (Variables|Default|GetTextRender) (Math|Vector|MakeVector 0.0 0.0 (Variables|Default|GetSizeInCm)) false false)
  (Rendering|Components|TextRender|SetText (Variables|Default|GetTextRender) (Utilities|Text|FormatText "{size} cm" (Variables|Default|GetSizeInCm))))