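; BP_DecalPrefab is a configurable decal prefab from the level design toolkit, exposing its look as Blueprint variables.
; Its construction script creates a dynamic material instance on the decal and pushes mask, color, roughness, normal, opacity and edge fade settings into material parameters.
; It has no runtime logic, as its event graph holds only disabled placeholder events.
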(event EventBeginPlay)

(event Collision|EventActorBeginOverlap
  (params (OtherActor :type Actor%20Object%20Reference)))

(event EventTick
  (params (DeltaSeconds :type Float%20%28single-precision%29)))

(fn ConstructionScript
  (bind _returnvalue (Rendering|Material|CreateDynamicMaterialInstance (Variables|Default|GetDecalActor) :!class /Script/Engine.DecalComponent))
  (Rendering|Material|SetTextureParameterValue _returnvalue "TextureMask" (Variables|Default|GetDecalMask))
  (Rendering|Material|SetTextureParameterValue _returnvalue "TextureColor" (Variables|Default|GetColorTexture))
  (Rendering|Material|SetVectorParameterValue _returnvalue "Color" (Variables|Default|GetColor) :!class /Script/Engine.MaterialInstanceDynamic)
  (Rendering|Material|SetScalarParameterValue _returnvalue "RoughnessMulti" (Variables|Default|GetRoughnessStrength) :!class /Script/Engine.MaterialInstanceDynamic)
  (Rendering|Material|SetTextureParameterValue _returnvalue "Roughness" (Variables|Default|GetRoughness%20Texture))
  (Rendering|Material|SetScalarParameterValue _returnvalue "Fade" (Variables|Default|GetEdgeFadeStrength) :!class /Script/Engine.MaterialInstanceDynamic)
  (Rendering|Material|SetScalarParameterValue _returnvalue "OpacityMulti" (Variables|Default|GetOpacity) :!class /Script/Engine.MaterialInstanceDynamic)
  (Rendering|Material|SetTextureParameterValue _returnvalue "Normal" (Variables|Default|GetNormal)))